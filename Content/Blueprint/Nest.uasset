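; Nest actor that displays its Id, spawns a single BP_Goblin at its sphere on request and drives that goblin's movement.
; Three externally triggered logic events set the pattern: delayed steady walk, timed stop-and-go, or forward walk with a brief 180-degree backtrack.
; Patterns set the goblin's animation and direction flags, using looping timers for the latter two.
; The IsCelebrate anim flag blocks the steady walk's start and clears either timer.
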(event `self.ReceiveBeginPlay`
  (`TextRenderComponent.K2_SetText` (`self.TextRender`) (`self.Id`)))

(event `self.ReceiveTick`
  (params (DeltaSeconds :type "Float (single-precision)")))

(event `Spawn_Goblin`
  ;[1 1 1] Создание гоблина на спавне
  (if (not (`self.isSpawned`))
    (set `self.isSpawned` true)
    (bind _returnvalue (`|SpawnActorFromClass` "/Game/Blueprint/BP_Goblin.BP_Goblin_C" (`KismetMathLibrary.MakeTransform` (`SceneComponent.K2_GetComponentLocation` (`self.Sphere`)) (`SceneComponent.K2_GetComponentRotation` (`self.StaticMeshComponent`))) "Undefined" "OverrideRootScale" null null))
    (set `self.Goblin` _returnvalue)))

(event `First_Logic`
  (bind _goblin (`self.Goblin`))
  (bind _myanim_bp (`/Game/Blueprint/BP_Goblin.MyAnim_BP` _goblin))
  ;[1 1 1] Идти вперёд
  (`KismetSystemLibrary.Delay` 1.5)
  (if (not (`/Game/Blueprint/ABD_Goblin.isCelebrate` _myanim_bp))
    (set `/Game/Blueprint/ABD_Goblin.isWalking` true _myanim_bp)
    (`/Game/Blueprint/BP_Goblin.Move_Forward` _goblin)))

(event `Second_Logic`
  ;[1 1 1] Идти вперёд 1 секунду, пол секунды стоп
  (bind _returnvalue (`KismetSystemLibrary.K2_SetTimerDelegate` (delegate `Move_Goblin`) 1.0 true)))

(event `Move_Goblin`
  (bind _myanim_bp (`/Game/Blueprint/BP_Goblin.MyAnim_BP` (`self.Goblin`)))
  ;[1 1 1] Идти вперёд 1 секунду, пол секунды стоп
  (if (`/Game/Blueprint/ABD_Goblin.isCelebrate` _myanim_bp)
    (`KismetSystemLibrary.K2_ClearAndInvalidateTimerHandle` (stale `Second_Logic` _returnvalue))
    (else
      (set `/Game/Blueprint/ABD_Goblin.isWalking` false _myanim_bp)
      (`KismetSystemLibrary.Delay` 0.5)
      (set `/Game/Blueprint/ABD_Goblin.isWalking` true _myanim_bp))))

(event `Third_Logic`
  ;[1 1 1] Идти вперёд 1 секунду, пол секунды назад
  (bind _returnvalue (`KismetSystemLibrary.K2_SetTimerDelegate` (delegate `Move_Gob`) 1.5 true)))

(event `Move_Gob`
  (bind _goblin (`self.Goblin`))
  (bind (_returnvalue_roll _returnvalue_pitch _returnvalue_yaw) (`KismetMathLibrary.BreakRotator` (`self.K2_GetActorRotation` _goblin)))
  (bind _myanim_bp (`/Game/Blueprint/BP_Goblin.MyAnim_BP` _goblin))
  (bind _returnvalue (`KismetMathLibrary.MakeRotator` 0.0 0.0 (+ _returnvalue_yaw 180.0)))
  ;[1 1 1] Идти вперёд 1 секунду, пол секунды назад
  (if (`/Game/Blueprint/ABD_Goblin.isCelebrate` _myanim_bp)
    (`KismetSystemLibrary.K2_ClearAndInvalidateTimerHandle` (stale `Third_Logic` _returnvalue))
    (else
      (set `/Game/Blueprint/ABD_Goblin.isWalking` true _myanim_bp)
      (set `/Game/Blueprint/BP_Goblin.isForward` true _goblin)
      (`KismetSystemLibrary.Delay` 1.0)
      (set `/Game/Blueprint/BP_Goblin.isForward` false _goblin)
      (`self.K2_SetActorRotation` _goblin _returnvalue false)
      (`KismetSystemLibrary.Delay` 0.46)
      (`self.K2_SetActorRotation` _goblin _returnvalue false))))

(fn `UserConstructionScript`)