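; BP_Goblin is a goblin enemy actor that walks along the world Y axis and celebrates when it reaches a Finish_Cube.
; While the cached ABD_Goblin anim instance flags walking, Tick moves the Sphere component forward or back according to IsForward, using short MoveComponentTo steps scaled by Speed.
; Overlapping the finish plays a sound, switches the animation flags from walking to celebrating, and destroys the actor after a delay.
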(event `self.ReceiveBeginPlay`
  (bind _asabd_goblin (cast `/Game/Blueprint/ABD_Goblin` (`SkeletalMeshComponent.GetAnimInstance` (`self.SM_EnemyGoblin`))))
  (set `self.MyAnim_BP` _asabd_goblin))

(event `self.ReceiveActorBeginOverlap`
  (params (OtherActor :type "Actor Object Reference"))
  (bind _myanim_bp (`self.MyAnim_BP`))
  ;[1 1 1] Проигрывание анимации при сталкивании с точкой финиша
  (cast `/Game/Blueprint/Finish_Cube` OtherActor)
  (`GameplayStatics.PlaySound2D` "/Game/Audio/FinishSound.FinishSound" 1.0 1.0 0.0 null null)
  (set `/Game/Blueprint/ABD_Goblin.isWalking` false _myanim_bp)
  (set `/Game/Blueprint/ABD_Goblin.isCelebrate` true _myanim_bp)
  (`KismetSystemLibrary.Delay` 10.0)
  (`self.K2_DestroyActor`))

(event `self.ReceiveTick`
  (params (DeltaSeconds :type "Float (single-precision)"))
  (if (`/Game/Blueprint/ABD_Goblin.isWalking` (`self.MyAnim_BP`))
    (if (`self.isForward`)
      (`self.Move_Forward`)
      (else
        (`self.Move_Back`)))))

(event `Move_Forward`
  (bind _y (.y (`SceneComponent.K2_GetComponentLocation` (`self.Sphere`))))
  ;[1 1 1] Move Forward
  (`KismetSystemLibrary.MoveComponentTo` (`self.Sphere`) (`KismetMathLibrary.MakeVector` (.x (`SceneComponent.K2_GetComponentLocation` (`self.Sphere`))) (`KismetMathLibrary.Lerp` _y (+ _y (`self.Speed`)) 0.1) (.z (`SceneComponent.K2_GetComponentLocation` (`self.Sphere`)))) (`SceneComponent.K2_GetComponentRotation` (`self.Sphere`)) true false 0.1))

(event `Move_Back`
  (bind _y (.y (`SceneComponent.K2_GetComponentLocation` (`self.Sphere`))))
  ;[1 1 1] Move Back
  (`KismetSystemLibrary.MoveComponentTo` (`self.Sphere`) (`KismetMathLibrary.MakeVector` (.x (`SceneComponent.K2_GetComponentLocation` (`self.Sphere`))) (`KismetMathLibrary.Lerp` _y (- _y (`self.Speed`)) 0.1) (.z (`SceneComponent.K2_GetComponentLocation` (`self.Sphere`)))) (`SceneComponent.K2_GetComponentRotation` (`self.Sphere`)) true false 0.1))

(fn `UserConstructionScript`)